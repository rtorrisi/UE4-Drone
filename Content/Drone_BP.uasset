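; Quadcopter drone Blueprint that simulates flight by applying physics forces at four engine positions on the Plane component.
; Each tick, every engine pushes along its forward vector, scaled by its PWM value and a shared K, then prints PWM values and rotation for debugging.
; Input sets pitch and roll targets and toggles Thrust with Space, but this graph never feeds them into the PWM values.
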(event `self.ReceiveTick`
  (params (DeltaSeconds :type "Float (single-precision)"))
  (bind _plane (`self.Plane`))
  (bind _engine1 (`self.Engine1`))
  (bind _engine4 (`self.Engine4`))
  (bind _engine3 (`self.Engine3`))
  (bind _engine2 (`self.Engine2`))
  (`PrimitiveComponent.AddForceAtLocationLocal` _plane (* (`SceneComponent.GetForwardVector` _engine2) (* (`self.PWM2`) (`self.K`))) (`SceneComponent.RelativeLocation` _engine2) "None")
  (`PrimitiveComponent.AddForceAtLocationLocal` _plane (* (`SceneComponent.GetForwardVector` _engine3) (* (`self.PWM3`) (`self.K`))) (`SceneComponent.RelativeLocation` _engine3) "None")
  (`PrimitiveComponent.AddForceAtLocationLocal` (`self.Plane`) (* (`SceneComponent.GetForwardVector` _engine4) (* (`self.PWM4`) (`self.K`))) (`SceneComponent.RelativeLocation` _engine4) "None")
  (`PrimitiveComponent.AddForceAtLocationLocal` (`self.Plane`) (* (`SceneComponent.GetForwardVector` _engine1) (* (`self.PWM1`) (`self.K`))) (`SceneComponent.RelativeLocation` _engine1) "None")
  (`KismetSystemLibrary.PrintString` (`KismetStringLibrary.Concat_StrStr` "PWM1: " (`KismetStringLibrary.Conv_DoubleToString` (`self.PWM1`)) " PWM2: " (`KismetStringLibrary.Conv_DoubleToString` (`self.PWM2`)) " PWM3: " (`KismetStringLibrary.Conv_DoubleToString` (`self.PWM3`)) " PWM4: " (`KismetStringLibrary.Conv_DoubleToString` (`self.PWM4`))) true true (struct :`G` 0.66 :`B` 1.0 :`A` 1.0) 0.0)
  (`KismetSystemLibrary.PrintString` (`KismetStringLibrary.Conv_RotatorToString` (`self.K2_GetActorRotation`)) true true (struct :`G` 0.66 :`B` 1.0 :`A` 1.0) 0.0))

(event `InputAxis|PitchControl`
  (params (AxisValue :type "Float (single-precision)"))
  (set `self.PitchTarget` (* AxisValue 1.0)))

(event `InputAxis|RollControl`
  (params (AxisValue :type "Float (single-precision)"))
  (set `self.RollTarget` (* AxisValue 1.0)))

(event `Key|SpaceBar`
  (params (Key :type "Key Structure"))
  (:`Pressed`
    (set `self.Thrust` 200.0))
  (:`Released`
    (set `self.Thrust` 0.0)))

(fn `UserConstructionScript`)